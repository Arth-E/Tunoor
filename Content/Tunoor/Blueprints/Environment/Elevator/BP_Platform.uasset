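; BP_Platform is an elevator platform that moves between an initial and a final position when activated as a target.
; BeginPlay converts both configured positions through the root's relative transform, and a timeline curve lerps the root between them.
; Activation plays the timeline and deactivation reverses it, while the construction script places the Platform component at the initial position.
; Its interaction functions are stubs returning fixed values or nothing.
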(event EventBeginPlay
  (bind _positions (Variables|Default|GetPositions))
  (bind _defaultsceneroot (Variables|Default|GetDefaultSceneRoot))
  (bind (_initialposition _finalposition) (Utilities|Struct|BreakST_Elevator_Struct _positions))
  (bind _returnvalue (Transformation|GetRelativeTransform _defaultsceneroot))
  (Variables|Default|SetVector_Initial (Math|Transform|TransformLocation _returnvalue _initialposition))
  (Variables|Default|SetVector_Target (Math|Transform|TransformLocation _returnvalue _finalposition)))

(event EventActivateTarget
  (bind _elevator_curve (Timeline|T_Elevator Play)
    (:Update
      (Transformation|SetWorldLocation (Variables|Default|GetDefaultSceneRoot) (Math|Vector|Lerp(Vector) (Variables|Default|GetVector_Initial) (Variables|Default|GetVector_Target) _elevator_curve) false false))))

(event EventDeactivateTarget
  (bind _elevator_curve (Timeline|T_Elevator Reverse)
    (:Update
      (Transformation|SetWorldLocation (Variables|Default|GetDefaultSceneRoot) (Math|Vector|Lerp(Vector) (Variables|Default|GetVector_Initial) (Variables|Default|GetVector_Target) _elevator_curve) false false))))

(fn ConstructionScript
  (Transformation|SetWorldLocation (Variables|Default|GetPlatform) (Math|Transform|TransformLocation (Transformation|GetRelativeTransform (Variables|Default|GetDefaultSceneRoot)) (.InitialPosition (Utilities|Struct|BreakST_Elevator_Struct (Variables|Default|GetPositions)))) false false))

(fn GetInteractionType
  (return "NewEnumerator0"))

(fn OnEnterInteractRange
  (return false))

(fn OnPushingStart
  (params (Instigator :type Actor%20Object%20Reference))
  (return 0 ""))