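; A pushable block interactable that the player moves along a single world axis.
; Each interaction step offsets it by rounded player input on the interactor's dominant facing axis, scaled by PushFactor.
; Movement is unswept; impact normals from stationary box and player-capsule traces, which ignore light sources, are added to the direction as collision pushback.
; When interaction ends, a box trace attaches the block to any BP_Platform it hits.
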(event EventBeginPlay
  (|CallParentFunction)
  (bind _outactors (Actor|GetAllActorsOfClass "/Game/Tunoor/Blueprints/Environment/Interactive/BP_LightSource.BP_LightSource_C"))
  (Variables|Default|SetLightSources _outactors))

(event Collision|EventActorBeginOverlap
  (params (OtherActor :type Actor%20Object%20Reference)))

(event EventTick
  (params (DeltaSeconds :type Float%20%28single-precision%29))
  (|CallParentFunction DeltaSeconds))

(event EventEndInteraction
  (bind _defaultsceneroot (Variables|Default|GetDefaultSceneRoot))
  (bind _returnvalue (Transformation|GetWorldLocation _defaultsceneroot))
  (bind _outhit (Collision|BoxTraceByChannel _returnvalue _returnvalue "100.000000,100.000000,100.000000" "0, 0, 0" "TraceTypeQuery1" false (Utilities|Array|MakeArray (Game|GetPlayerCharacter 0)) "Persistent"))
  (if (.bBlockingHit (Collision|BreakHitResult _outhit))
    (bind _asbp_elevator_1 (Utilities|Casting|CastToBP_Platform (.HitActor (Collision|BreakHitResult _outhit))))
    (Transformation|AttachActorToActor _asbp_elevator_1 "None" "KeepWorld" "KeepWorld" "KeepWorld" true)))

(event EventOnPlayerInteraction
  (bind _pushabledirection (CallFunction|GetDirection))
  (bind _output_get (Variables|Default|SetCurrentLocation (Transformation|GetActorLocation)))
  (Transformation|SetWorldLocation (Variables|Default|GetDefaultSceneRoot) (+ _output_get (* (+ _pushabledirection (CallFunction|GetCollision)) (Variables|Default|GetPushFactor))) false false))

(fn ConstructionScript
  (|CallParentFunction))

(fn InitializeInteraction
  (|CallParentFunction))

(fn GetDirection
  (bind _interactordata (Variables|Default|GetInteractorData))
  (bind (_x _y) (Math|Vector|BreakVector (.interactorinputvector _interactordata)))
  (bind (_x_2 _y_2) (Math|Vector|BreakVector (.interactorforward _interactordata)))
  (LocalVariables|SetX _x)
  (LocalVariables|SetY _y)
  (if (> (Math|Float|Absolute(Float) _x_2) (Math|Float|Absolute(Float) _y_2))
    (LocalVariables|SetY 0.0)
    (else
      (LocalVariables|SetX 0.0)))
  (return (Math|Vector|MakeVector (Math|Conversions|ToFloat(Integer) (Math|Float|Round (LocalVariables|GetX))) (Math|Conversions|ToFloat(Integer) (Math|Float|Round (LocalVariables|GetY))) 0.0)))

(fn GetCollision
  (bind _returnvalue (Transformation|GetActorLocation))
  (bind _returnvalue_2 (Game|GetPlayerCharacter 0))
  (bind _lightsources (Variables|Default|GetLightSources))
  (bind _capsulecomponent (Variables|/Script/Engine.Character|GetCapsuleComponent _returnvalue_2))
  (bind _returnvalue_3 (Transformation|GetWorldLocation _capsulecomponent))
  (Rendering|Debug|FlushPersistentDebugLines)
  (bind _outhit (Collision|BoxTraceByChannel _returnvalue _returnvalue (/ (.boxextent (StaticMesh|GetBounds (Variables|/Script/Engine.StaticMeshComponent|GetStaticMesh (Variables|Default|GetCube)))) 1.15) "0, 0, 0" "TraceTypeQuery1" false _lightsources "None"))
  (bind _outhit_2 (Collision|CapsuleTraceByChannel _returnvalue_3 _returnvalue_3 (/ (.SphereRadius (Collision|GetComponentBounds _capsulecomponent)) 4.5) (Variables|/Script/Engine.CapsuleComponent|GetCapsuleHalfHeight _capsulecomponent) "TraceTypeQuery1" false _lightsources "ForDuration"))
  (return (+ (.ImpactNormal (Collision|BreakHitResult _outhit)) (.ImpactNormal (Collision|BreakHitResult _outhit_2)))))