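; BP_ChildRotating_Canon is a child interactive environment Blueprint for a cannon that the player rotates by interacting with it.
; On each player interaction event, it adds local yaw from the interactor's X input, scaled by the Y component of RotationSpeed and world delta time.
; BeginPlay, construction and interaction initialization only call the parent implementations.
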(event EventBeginPlay
  (|CallParentFunction))

(event Collision|EventActorBeginOverlap
  (params (OtherActor :type Actor%20Object%20Reference)))

(event EventOnPlayerInteraction
  (Transformation|AddActorLocalRotation (Math|Rotator|MakeRotator 0.0 0.0 (.y (* (Variables|Default|GetRotation%20Speed) (Utilities|Time|GetWorldDeltaSeconds) (.x (.interactorinputvector (Variables|Default|GetInteractorData)))))) false false))

(fn ConstructionScript
  (|CallParentFunction))

(fn InitializeInteraction
  (|CallParentFunction))