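; BP_LightCanon is an interactive environment object with the beginnings of a player push mechanic.
; OnInteract runs a FlipFlop whose A side calls CanPush, a short forward trace from the player that must hit this actor.
; Success sets IsPushing; failure clears it, zeroes PushDirection and detaches the player into walking mode.
; No movement or attach logic exists here, the B side is unwired, and OnEnterInteractRange returns false.
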(event EventBeginPlay
  (if (Variables|Default|GetIsPushing)
    _))

(event EventOnInteract
  (Utilities|FlowControl|FlipFlop
    (:A
      (bind _canpush (CallFunction|CanPush))
      (if _canpush
        (Variables|Default|SetIsPushing true)
        (else
          (Variables|Default|SetIsPushing false)
          (Variables|Default|SetPushDirection "0, 0, 0")
          (CallFunction|DetachPlayer))))))

(fn ConstructionScript)

(fn CanPush
  (bind _returnvalue (Game|GetPlayerCharacter 0))
  (bind _returnvalue_2 (Transformation|GetActorLocation _returnvalue))
  (bind (_outhit _returnvalue_3) (Collision|LineTraceByChannel _returnvalue_2 (+ _returnvalue_2 (* (Transformation|GetActorForwardVector _returnvalue) 1e+02)) "TraceTypeQuery1" false (Utilities|Array|MakeArray _returnvalue) "None" false))
  (if _returnvalue_3
    (return (== (.HitActor (Collision|BreakHitResult _outhit)) self))))

(fn DetachPlayer
  (bind _returnvalue (Game|GetPlayerCharacter 0))
  (Pawn|Components|CharacterMovement|SetMovementMode (Variables|/Script/Engine.Character|GetCharacterMovement _returnvalue) "MOVE_Walking" 0)
  (Transformation|DetachFromActor _returnvalue "KeepWorld" "KeepWorld" "KeepWorld"))

(fn OnEnterInteractRange
  (return false))