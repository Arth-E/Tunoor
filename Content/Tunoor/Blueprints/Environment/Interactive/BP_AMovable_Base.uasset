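; Base Blueprint for interactive movable objects that the player can grab and push, with empty start, update and end hooks apparently meant for child classes.
; Interacting toggles pushing: it attaches the player and disables their movement, then detaches and restores walking.
; While pushing, Tick refreshes interactor input, transform and camera data before calling the update hook.
; Trace helpers test whether the player faces it and whether its space is clear, but are uncalled here.
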(event Custom|End%20Interaction)

(event Custom|OnPlayerInteraction)

(event EventTick
  (params (DeltaSeconds :type Float%20%28single-precision%29))
  (if (Variables|Default|GetIsPushing)
    (CallFunction|SetInteractorData)
    (CallFunction|OnPlayerInteraction)))

(event EventOnInteract
  (bind _returnvalue (Game|GetPlayerCharacter 0))
  ;[1 1 1] Fonction OnInteract
  (Utilities|FlowControl|FlipFlop
    (:A
      (if (not (Variables|Default|GetIsPushing))
        (Variables|Default|SetIsPushing true)
        (CallFunction|InitializeInteraction)
        (Transformation|AttachActorToActor _returnvalue self "None" "KeepWorld" "KeepWorld" "KeepWorld" true)
        (Pawn|Components|CharacterMovement|DisableMovement (Variables|/Script/Engine.Character|GetCharacterMovement _returnvalue))))
    (:B
      (Variables|Default|SetIsPushing false)
      (CallFunction|DetachPlayer)
      (CallFunction|EndInteraction))))

(fn ConstructionScript)

(fn CanPush
  (bind _returnvalue (Game|GetPlayerCharacter 0))
  (bind _returnvalue_2 (Transformation|GetActorLocation _returnvalue))
  (bind (_outhit _returnvalue_3) (Collision|LineTraceByChannel _returnvalue_2 (+ _returnvalue_2 (* (Transformation|GetActorForwardVector _returnvalue) 1e+02)) "TraceTypeQuery1" false (Utilities|Array|MakeArray _returnvalue) "None" false))
  (if _returnvalue_3
    (return (== (.HitActor (Collision|BreakHitResult _outhit)) self))))

(fn SetInteractorData
  (bind _returnvalue (Game|GetPlayerCharacter 0))
  (bind _asbp_player_test (Utilities|Casting|CastToBP_Player_Test _returnvalue))
  (Variables|Default|SetInteractorData (Utilities|Struct|MakeS_InteractorData (Pawn|Components|PawnMovement|GetLastInputVector (Pawn|GetMovementComponent _returnvalue)) (Transformation|GetActorForwardVector _returnvalue) (Transformation|GetActorLocation _returnvalue) (Default|GetCamera _asbp_player_test) _asbp_player_test)))

(fn DetachPlayer
  (bind _returnvalue (Game|GetPlayerCharacter 0))
  (Pawn|Components|CharacterMovement|SetMovementMode (Variables|/Script/Engine.Character|GetCharacterMovement _returnvalue) "MOVE_Walking" 0)
  (Transformation|DetachFromActor _returnvalue "KeepWorld" "KeepWorld" "KeepWorld"))

(fn CheckCollision
  (bind _returnvalue (Transformation|GetActorLocation))
  (Rendering|Debug|FlushPersistentDebugLines)
  (bind _returnvalue_2 (Collision|BoxTraceByChannel _returnvalue _returnvalue (/ (.boxextent (StaticMesh|GetBounds (Variables|/Script/Engine.StaticMeshComponent|GetStaticMesh (Variables|Default|GetCube)))) 1.3) "0, 0, 0" "TraceTypeQuery1" false 0 "Persistent"))
  (return (not _returnvalue_2)))

(fn InitializeInteraction)

(fn LightTouch
  (return))

(fn OnEnterInteractRange
  (return true))