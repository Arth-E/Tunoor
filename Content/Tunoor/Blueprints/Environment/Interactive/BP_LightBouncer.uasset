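; BP_LightBouncer is an interactive object that relays light through a child BP_LightSource actor.
; When a light source enters its box, it re-fires that source's ray, then activates the child and fires its ray.
; When one leaves, it re-fires that source's ray, then deactivates the child and cancels its ray.
; Player interaction runs the parent logic, then re-fires the child's ray if IsPushing is set.
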(event OnComponentBeginOverlap(Box)
  (params (OverlappedComponent :type Primitive%20Component%20Object%20Reference) (OtherActor :type Actor%20Object%20Reference) (OtherComp :type Primitive%20Component%20Object%20Reference) (OtherBodyIndex :type Integer) (bFromSweep :type Boolean) (SweepResult :type Hit%20Result%20Structure%20%28by%20ref%29))
  (bind _asbp_light_source (Utilities|Casting|CastToBP_LightSource OtherActor))
  (Default|RayEvent _asbp_light_source)
  (bind _asbp_light_source_2 (Utilities|Casting|CastToBP_LightSource (Variables|/Script/Engine.ChildActorComponent|GetChildActor (Variables|Default|GetChildLightSource))))
  (Development|PrintString "Reactivated")
  (Variables|/Game/Tunoor/Blueprints/Environment/Interactive/BP_LightSource.BP_LightSource_C|SetbIsActivated _asbp_light_source_2 true)
  (Default|RayEvent _asbp_light_source_2))

(event OnComponentEndOverlap(Box)
  (params (OverlappedComponent :type Primitive%20Component%20Object%20Reference) (OtherActor :type Actor%20Object%20Reference) (OtherComp :type Primitive%20Component%20Object%20Reference) (OtherBodyIndex :type Integer))
  (bind _asbp_light_source (Utilities|Casting|CastToBP_LightSource OtherActor))
  (Default|RayEvent _asbp_light_source)
  (bind _asbp_light_source_2 (Utilities|Casting|CastToBP_LightSource (Variables|/Script/Engine.ChildActorComponent|GetChildActor (Variables|Default|GetChildLightSource))))
  (Development|PrintString "Deactivated")
  (Variables|/Game/Tunoor/Blueprints/Environment/Interactive/BP_LightSource.BP_LightSource_C|SetbIsActivated _asbp_light_source_2 false)
  (Default|CancelRay _asbp_light_source_2))

(event EventBeginPlay
  (|CallParentFunction) ; This node is disabled and will not be called.\nDrag off pins to build functionality.
)

(event Collision|EventActorBeginOverlap
  (params (OtherActor :type Actor%20Object%20Reference))
  (|CallParentFunction OtherActor) ; This node is disabled and will not be called.\nDrag off pins to build functionality.
)

(event EventOnPlayerInteraction
  (Utilities|FlowControl|Sequence
    (:then_0
      (|CallParentFunction))
    (:then_1
      (if (Variables|Default|GetIsPushing)
        (bind _asbp_light_source (Utilities|Casting|CastToBP_LightSource (Variables|/Script/Engine.ChildActorComponent|GetChildActor (Variables|Default|GetChildLightSource))))
        (Default|RayEvent _asbp_light_source)))))

(fn ConstructionScript
  (|CallParentFunction))