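; BP_LightSource is an interactive environment actor that emits a visible light ray along its arrow when activated.
; On BeginPlay or RayEvent, an active source line-traces forward, ignoring all light sources, and stretches the ray mesh's Z scale to the hit distance or full length.
; An inactive source hides the ray at BeginPlay by flattening its Y scale.
; Interaction functions like LightTouch and OnPushingStart are stubs.
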(event Custom|Cancel%20Ray
  (CallFunction|DeactivateRay))

(event Custom|Initialise%20Ray%20Length
  (CallFunction|SetRayLength (Variables|Default|GetRay%20Length)))

(event Custom|RayEvent
  (if (Variables|Default|GetbIsActivated)
    (bind (_bblockinghit _distance) (CallFunction|RayLogic (Variables|Default|GetRay%20Length)))
    (if _bblockinghit
      (CallFunction|SetRayLength _distance)
      (else
        (CallFunction|InitialiseRayLength)))))

(event EventBeginPlay
  (bind _outactors (Actor|GetAllActorsOfClass "BP_LightSource_C"))
  (Variables|Default|SetLight%20Sources _outactors)
  (if (Variables|Default|GetbIsActivated)
    (CallFunction|RayEvent)
    (else
      (CallFunction|CancelRay))))

(fn ConstructionScript)

(fn SetRayLength
  (params (Length :type Float%20%28double-precision%29))
  (bind _ray (Variables|Default|GetRay))
  (bind _returnvalue (Transformation|GetWorldScale _ray))
  (Transformation|SetWorldScale3D _ray (Math|Vector|MakeVector (.x _returnvalue) (.y _returnvalue) (/ Length 1e+02))))

(fn RayLogic
  (params (Ray%20Length :type Float%20%28double-precision%29))
  (bind _arrow (Variables|Default|GetArrow))
  (bind _returnvalue (Transformation|GetWorldLocation _arrow))
  (bind _outhit (Collision|LineTraceByChannel _returnvalue (+ _returnvalue (* (Math|Vector|GetForwardVector _arrow) Ray%20Length)) "TraceTypeQuery1" false (Variables|Default|GetLight%20Sources) "Persistent"))
  (return (.bBlockingHit (Collision|BreakHitResult _outhit)) (.Distance (Collision|BreakHitResult _outhit))))

(fn DeactivateRay
  (bind _ray (Variables|Default|GetRay))
  (bind _returnvalue (Transformation|GetWorldScale _ray))
  (Transformation|SetWorldScale3D _ray (Math|Vector|MakeVector (.x _returnvalue) 0.0 (.z _returnvalue))))

(fn GetInteractionType
  (return "NewEnumerator0"))

(fn LightTouch
  (return))

(fn OnEnterInteractRange
  (return false))

(fn OnPushingStart
  (params (Instigator :type Actor%20Object%20Reference))
  (return 0 ""))