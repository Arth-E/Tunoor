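; Light source component that fits a visible ray to whatever blocks it.
; SetRayComponents stores the ray and arrow, then runs a Visibility line trace from the arrow along its unscaled forward vector.
; A hit sets the ray's Y scale from the hit distance and resets a DoOnce gate.
; A miss restores the default length once through that gate and prints a debug message.
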(event Custom|Initialize%20Ray%20Length
  (Utilities|FlowControl|DoOnce false
    (:Completed
      (CallFunction|SetRayLength (Variables|Default|GetRay_Length))
      (Development|PrintString "Out of touch"))))

(event Custom|RayEvent
  (bind (_blocking_hit _distance) (CallFunction|RayLogic))
  (if _blocking_hit
    (CallFunction|SetRayLength _distance)
    (CallFunction|ResetRayLength)
    (else
      (CallFunction|InitializeRayLength))))

(event Custom|ResetRayLength
  (Utilities|FlowControl|DoOnce false) ; enters at Reset
)

(event Custom|Set%20Ray%20Components
  (params (Ray :type Scene%20Component%20Object%20Reference) (Arrow :type Scene%20Component%20Object%20Reference))
  (Variables|Default|SetRay Ray)
  (Variables|Default|SetArrow Arrow)
  (CallFunction|RayEvent))

(fn RayLogic
  (bind _arrow (Variables|Default|GetArrow))
  (bind _returnvalue (Transformation|GetWorldLocation _arrow))
  (bind _outhit (Collision|LineTraceByChannel _returnvalue (+ _returnvalue (Math|Vector|GetForwardVector _arrow)) "TraceTypeQuery1" false 0 "None"))
  (return (.bBlockingHit (Collision|BreakHitResult _outhit)) (.Distance (Collision|BreakHitResult _outhit))))

(fn SetRayLength
  (params (RayLength :type Float%20%28double-precision%29) (NewParam :type Scene%20Capture%20Component%20Cube%20Object%20Reference))
  (bind _ray (Variables|Default|GetRay))
  (bind _returnvalue (Transformation|GetWorldScale _ray))
  (bind (_x _y _z) (Math|Vector|BreakVector _returnvalue))
  (Transformation|SetWorldScale3D _ray (Math|Vector|MakeVector _x (/ RayLength 1e+02) _z)))