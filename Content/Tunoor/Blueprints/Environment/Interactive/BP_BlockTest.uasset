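; BP_BlockTest is an interactable pushable block that can snap onto a target position, such as a plate.
; On push start it picks the arrow component (right, left, front or back) nearest the instigator and returns that transform for alignment, plus MovingBlock to grab.
; Ending the push resets the cached closest point and distance.
; SnapToPlate uses a timeline to lerp the actor to the given target without sweeping.
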(event Custom|SnapToPlate
  (params (Target :type Vector))
  (Variables|Default|SetStart%20Location (Transformation|GetActorLocation))
  (bind _newtrack_0 (Timeline|SnapToTarget PlayFromStart)
    (:Update
      (Transformation|SetActorLocation (Math|Vector|Lerp(Vector) (Variables|Default|GetStart%20Location) Target _newtrack_0) false false))))

(event EventBeginPlay
  (Variables|Default|SetArrows (Utilities|Array|MakeArray (Variables|Default|GetArrowRight) (Variables|Default|GetArrowLeft) (Variables|Default|GetArrowFront) (Variables|Default|GetArrowBack))))

(event Collision|EventActorBeginOverlap
  (params (OtherActor :type Actor%20Object%20Reference)))

(event EventTick
  (params (DeltaSeconds :type Float%20%28single-precision%29)))

(event EventOnInteract)

(event EventOnPushingEnd
  (CallFunction|PushingEnd))

(fn ConstructionScript)

(fn PushingEnd
  (Variables|Default|SetClosestDistance 9999.0)
  (Variables|Default|SetClosest%20Point 0))

(fn GetInteractionType
  (return "NewEnumerator0"))

(fn OnEnterInteractRange
  (return true))

(fn OnPushingStart
  (params (Instigator :type Actor%20Object%20Reference))
  (for _array_element (Variables|Default|GetArrows)
    (if (< (Math|Vector|Distance(Vector) (Transformation|GetWorldLocation _array_element) (Transformation|GetActorLocation Instigator)) (Variables|Default|GetClosestDistance))
      (Variables|Default|SetClosestDistance (Math|Vector|Distance(Vector) (Transformation|GetWorldLocation _array_element) (Transformation|GetActorLocation Instigator)))
      (Variables|Default|SetClosest%20Point _array_element)))
  (return (Variables|Default|GetMovingBlock) (Transformation|GetWorldTransform (Variables|Default|GetClosest%20Point))))