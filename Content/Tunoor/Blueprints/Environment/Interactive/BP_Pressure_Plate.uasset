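; Pressure plate that activates and deactivates a list of target actors when something enters or leaves its box trigger.
; A BP_Movable_block sets the Pressed flag, so other overlaps are ignored until a block leaves.
; When unpressed, any other actor activates the targets on entry and deactivates them on exit.
; Targets receive ActivateTargetMessage and DeactivateTargetMessage calls, looped over ActorsList.
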(event OnComponentBeginOverlap(Box)
  (params (OverlappedComponent :type Primitive%20Component%20Object%20Reference) (OtherActor :type Actor%20Object%20Reference) (OtherComp :type Primitive%20Component%20Object%20Reference) (OtherBodyIndex :type Integer) (bFromSweep :type Boolean) (SweepResult :type Hit%20Result%20Structure%20%28by%20ref%29))
  (if (not (Variables|Default|GetPressed))
    (Utilities|Casting|CastToBP_Movable_block OtherActor
      (:then
        (Variables|Default|SetPressed true)
        (CallFunction|ActivateActors))
      (:CastFailed
        (CallFunction|ActivateActors)))))

(event OnComponentEndOverlap(Box)
  (params (OverlappedComponent :type Primitive%20Component%20Object%20Reference) (OtherActor :type Actor%20Object%20Reference) (OtherComp :type Primitive%20Component%20Object%20Reference) (OtherBodyIndex :type Integer))
  (if (Variables|Default|GetPressed)
    (Utilities|Casting|CastToBP_Movable_block OtherActor)
    (Variables|Default|SetPressed false)
    (CallFunction|DeactivateActors)
    (else
      (CallFunction|DeactivateActors))))

(event Custom|ActivateActors
  (for _array_element (Variables|Default|GetActorsList)
    (Class|BPIInteract|ActivateTarget(Message) _array_element)))

(event Custom|DeactivateActors
  (for _array_element (Variables|Default|GetActorsList)
    (Class|BPIInteract|DeactivateTarget(Message) _array_element)))

(event EventBeginPlay)

(event Collision|EventActorBeginOverlap
  (params (OtherActor :type Actor%20Object%20Reference)))

(event EventTick
  (params (DeltaSeconds :type Float%20%28single-precision%29)))

(fn ConstructionScript)