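; BP_Elevator is an elevator actor that moves a platform between two configured positions when something overlaps its collision component.
; The construction script teleports the platform to the initial position.
; Any overlap prints a debug string and restarts a timeline, whose curve drives a world-space lerp toward the final position.
; There is no overlap filter or return trip, so each new overlap replays the movement from the start.
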(event OnComponentBeginOverlap(collision)
  (params (OverlappedComponent :type Primitive%20Component%20Object%20Reference) (OtherActor :type Actor%20Object%20Reference) (OtherComp :type Primitive%20Component%20Object%20Reference) (OtherBodyIndex :type Integer) (bFromSweep :type Boolean) (SweepResult :type Hit%20Result%20Structure%20%28by%20ref%29))
  (bind _positions (Variables|Default|GetPositions))
  (bind (_initialposition _finalposition) (Utilities|Struct|BreakST_Elevator_Struct _positions))
  (Development|PrintString "Passé")
  (bind _elevator_curve (Timeline|T_Elevator PlayFromStart)
    (:Update
      (Transformation|SetWorldLocation (Variables|Default|GetPlatform) (Math|Vector|Lerp(Vector) _initialposition _finalposition _elevator_curve) false false))))

(event EventBeginPlay)

(event Collision|EventActorBeginOverlap
  (params (OtherActor :type Actor%20Object%20Reference)))

(event EventTick
  (params (DeltaSeconds :type Float%20%28single-precision%29)))

(fn ConstructionScript
  (Transformation|SetWorldLocation (Variables|Default|GetPlatform) (.InitialPosition (Utilities|Struct|BreakST_Elevator_Struct (Variables|Default|GetPositions))) false true))